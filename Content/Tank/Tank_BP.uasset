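; Player-controllable tank Blueprint that binds input for driving, aiming the camera, firing and swapping views.
; On BeginPlay it hands the barrel and turret to TankAiming, both tracks to TankMovement, and itself to the health bar widget.
; Axis inputs rotate the azimuth gimbal and spring arm, and drive either per-track throttles or TankMovement's move and rotate intents.
; Fire calls TankAiming, and Swap Cam toggles third- and first-person cameras.
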(event EventBeginPlay
  (CallFunction|InitializeTankAiming)
  (CallFunction|InitializeTankMovement)
  (CallFunction|InitializeHealthBar))

(event Input|ActionEvents|InputActionFire
  (params (Key :type Key%20Structure))
  ;[1 1 1] Firing input binding
  (:Pressed
    (Class|TankAimingComponent|Fire (Variables|Default|GetTankAiming))))

(event Input|ActionEvents|InputActionSwapCam
  (params (Key :type Key%20Structure))
  ;[1 1 1] Camera swapping
  (:Pressed
    (Components|Activation|ToggleActive (Variables|Default|GetThird%20Person))
    (Components|Activation|ToggleActive (Variables|Default|GetFirst%20Person))))

(event Input|AxisEvents|InputAxisAimAzimuth
  (params (AxisValue :type Float%20%28single-precision%29))
  ;[1 1 1] Camera input binding
  (Transformation|AddLocalRotation (Variables|Default|GetAzimuth%20Gimbal) (Math|Rotator|MakeRotator 0.0 0.0 AxisValue) false false))

(event Input|AxisEvents|InputAxisMoveForward
  (params (AxisValue :type Float%20%28single-precision%29))
  ;[1 1 1] Movement input binding
  (Class|TankMovementComponent|IntendMoveForward (Variables|Default|GetTankMovement) AxisValue))

(event Input|AxisEvents|InputAxisAimElevation
  (params (AxisValue :type Float%20%28single-precision%29))
  ;[1 1 1] Camera input binding
  (Transformation|AddLocalRotation (Variables|Default|GetSpringArm) (Math|Rotator|MakeRotator 0.0 AxisValue 0.0) false false))

(event Input|AxisEvents|InputAxisLeftTrackThrottle
  (params (AxisValue :type Float%20%28single-precision%29))
  ;[1 1 1] Movement input binding
  (Class|TankTrack|SetThrottle (Variables|Default|GetTrack%20Left) AxisValue))

(event Input|AxisEvents|InputAxisRightTrackThrottle
  (params (AxisValue :type Float%20%28single-precision%29))
  ;[1 1 1] Movement input binding
  (Class|TankTrack|SetThrottle (Variables|Default|GetTrack%20Right) AxisValue))

(event Input|AxisEvents|InputAxisRotateTank
  (params (AxisValue :type Float%20%28single-precision%29))
  ;[1 1 1] Movement input binding
  (Class|TankMovementComponent|IntendRotate (Variables|Default|GetTankMovement) AxisValue))

(fn ConstructionScript)

(fn InitializeHealthBar
  (bind _ashealth_bar (Utilities|Casting|CastToHealthBar (UserInterface|GetUserWidgetObject (Variables|Default|GetWidget))))
  (Variables|/Game/UI/HealthBar.HealthBar_C|SetBP%20Tank%20Reference _ashealth_bar self))

(fn InitializeTankMovement
  (Class|TankMovementComponent|Initialize (Variables|Default|GetTankMovement) (Variables|Default|GetTrack%20Left) (Variables|Default|GetTrack%20Right)))

(fn InitializeTankAiming
  (Class|TankAimingComponent|Initialize (Variables|Default|GetTankAiming) (Variables|Default|GetTankBarrel) (Variables|Default|GetTankTurret)))